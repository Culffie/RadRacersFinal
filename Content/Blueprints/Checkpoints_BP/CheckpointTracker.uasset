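; Race manager that runs an ordered array of checkpoints and tracks lap and race completion through MyPlayerController.
; On BeginPlay it copies lap, save slot and default best-time settings to the controller, numbers the checkpoints, binds their cleared events and activates the first.
; Each clear reveals and enables the next checkpoint and moves the respawn point to the one just passed.
; The last checkpoint updates the lap and either loops or completes the race, triggering Restart.
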(event Custom|ApplySettings
  (bind _controllerreference (Variables|Default|GetControllerReference))
  ;[1 1 1] Applying the user settings
  (Variables|/Game/Blueprints/My_Player_Controller_BP/MyPlayerController.MyPlayerController_C|SetMaxLaps _controllerreference (Variables|LapSettings|GetMaxLaps))
  (Variables|/Game/Blueprints/My_Player_Controller_BP/MyPlayerController.MyPlayerController_C|SetSaveSlot _controllerreference (Variables|LapSettings|GetSaveGameName))
  (CallFunction|UpdateTimes)
  (Default|StartGameSetup (Variables|Default|GetControllerReference)))

(event Custom|StartSeq
  (bind _checkpoints (Variables|Checkpoints|GetCheckpoints))
  ;[1 1 1] Starting sequence - Getting all the checkpoints in game
  (for (_array_element _array_index) (Variables|Checkpoints|GetCheckpoints)
    (Variables|/Game/Blueprints/Checkpoints_BP/Checkpoint.Checkpoint_C|SetCheckpointNumber _array_element (+ _array_index 1))
    (Variables|Default|SetTotalCheckpoints (Utilities|Array|Length _checkpoints))
    (CallFunction|ActivateCheckpoint (Utilities|Array|Get(acopy) _checkpoints))
    (for _array_element_2 (Variables|Checkpoints|GetCheckpoints)
      (EventDispatchers|BindEventtoCheckpointCleared _array_element_2 (delegate Custom|CheckpointPassed)))))

(event Custom|CheckpointPassed
  (params (NextCheckpoint :type Integer))
  (bind _controllerreference (Variables|Default|GetControllerReference))
  ;[1 1 1] Check if checkpoints and race are clear
  (CallFunction|LapCheck NextCheckpoint)
  (if (Variables|/Game/Blueprints/My_Player_Controller_BP/MyPlayerController.MyPlayerController_C|GetRaceComplete _controllerreference)
    (Default|Restart _controllerreference)))

(event EventBeginPlay
  ;[1 1 1] Casting to the MyPlayerController tab
  (bind _asmy_player_controller (Utilities|Casting|CastToMyPlayerController (Game|GetPlayerController 0)))
  (Variables|Default|SetControllerReference _asmy_player_controller)
  (CallFunction|ApplySettings)
  (CallFunction|StartSeq))

(fn ConstructionScript)

(fn UpdateTimes
  (bind _controllerreference (Variables|Default|GetControllerReference))
  ;[1 1 1] Passing all the Times to MyPlayerController Times
  (Variables|/Game/Blueprints/My_Player_Controller_BP/MyPlayerController.MyPlayerController_C|SetDefaultBestLapTime _controllerreference (Variables|LapSettings|GetDefaultBestLap))
  (Variables|/Game/Blueprints/My_Player_Controller_BP/MyPlayerController.MyPlayerController_C|SetDefaultBestRaceTime _controllerreference (Variables|LapSettings|GetDefaultBestTime)))

(fn LapCheck
  (params (Checkpoint :type Integer))
  ;[1 1 1] Lap check script - Checks to see if we have completed race, a lap or sets up the next checkpoint
  (bind _output_get (LocalVariables|SetLocalCheckpoint Checkpoint))
  (if (== _output_get (Variables|Default|GetTotalCheckpoints))
    (bind _isracecomplete (CallFunction|RaceCompleteCheck))
    (if _isracecomplete
      _
      (else
        (CallFunction|ActivateCheckpoint (Utilities|Array|Get(acopy) (Variables|Checkpoints|GetCheckpoints)))))
    (Default|UpdateLap (Variables|Default|GetControllerReference))
    (else
      (CallFunction|ActivateCheckpoint (Utilities|Array|Get(acopy) (Variables|Checkpoints|GetCheckpoints) (LocalVariables|GetLocalCheckpoint)))))
  (Variables|/Game/Blueprints/My_Player_Controller_BP/MyPlayerController.MyPlayerController_C|SetRespawnLocation (Variables|Default|GetControllerReference) (Math|Transform|MakeTransform (.location (Transformation|GetActorTransform (Utilities|Array|Get(acopy) (Variables|Checkpoints|GetCheckpoints) (- (LocalVariables|GetLocalCheckpoint) 1)))) (.rotation (Transformation|GetActorTransform (Utilities|Array|Get(acopy) (Variables|Checkpoints|GetCheckpoints) (- (LocalVariables|GetLocalCheckpoint) 1)))) "1,1,1")))

(fn ActivateCheckpoint
  (params (NextCheckpoint :type Checkpoint%20Object%20Reference))
  ;[1 1 1] This will activate next checkpoint
  (Development|SetHiddeninGame (Variables|/Game/Blueprints/Checkpoints_BP/Checkpoint.Checkpoint_C|GetParticleSystem NextCheckpoint) false false)
  (Variables|/Script/Engine.PrimitiveComponent|SetbGenerateOverlapEvents (Variables|/Game/Blueprints/Checkpoints_BP/Checkpoint.Checkpoint_C|GetBoxTrigger NextCheckpoint) true))

(fn RaceCompleteCheck
  (bind _controllerreference (Variables|Default|GetControllerReference))
  (bind _controllerreference_2 (Variables|Default|GetControllerReference))
  ;[1 1 1] Rce complete check, sets race complete in player controller
  (if (>= (Variables|/Game/Blueprints/My_Player_Controller_BP/MyPlayerController.MyPlayerController_C|GetActualLap _controllerreference) (Variables|/Game/Blueprints/My_Player_Controller_BP/MyPlayerController.MyPlayerController_C|GetMaxLaps _controllerreference))
    (bind _output_get (Variables|/Game/Blueprints/My_Player_Controller_BP/MyPlayerController.MyPlayerController_C|SetRaceComplete _controllerreference_2 true))
    (LocalVariables|SetLocalComplete _output_get)
    (else
      (bind _output_get_2 (Variables|/Game/Blueprints/My_Player_Controller_BP/MyPlayerController.MyPlayerController_C|SetRaceComplete _controllerreference_2 false))
      (LocalVariables|SetLocalComplete _output_get_2)))
  (return (LocalVariables|GetLocalComplete)))