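; BP_HoverVehicleOld is a hover vehicle Blueprint containing helper functions for axis splitting and stuck detection, with an empty construction script.
; SplitAxis separates a signed value into clamped positive and negative magnitudes.
; RespawnCheck flags the vehicle as stuck when it is nearly stationary and tipped over, using a dot product of its up vector against world up.
; No event graph, movement or respawn logic appears here.
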(fn ConstructionScript)

(fn SplitAxis
  (params (Value :type Float%20%28single-precision%29))
  (return (Math|Float|Clamp(Float) Value) (Math|Float|Clamp(Float) (- 0.0 Value))))

(fn RespawnCheck
  ;[1 1 1] Checks to see if player is not moving and upside down
  (if (and (< (Math|Vector|DotProduct (Transformation|GetActorUpVector) "0, 0,1.000000") 0.5) (< (Variables|Default|GetCurrentSpeed) 0.5))
    (Variables|Default|SetStuck? true)
    (else
      (Variables|Default|SetStuck? false)))
  (return (Variables|Default|GetStuck?)))